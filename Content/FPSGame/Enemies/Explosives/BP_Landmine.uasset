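; Landmine hazard that explodes when the player touches it, in either a static or an activable variant set by LandmineType.
; The construction script places the mesh at rest height, or sunk below it for activable mines.
; On activable mines, player overlap with TrapActivator plays a one-shot timeline that raises the mesh.
; Box overlap spawns explosion effects, applies environmental damage and destroys the box and mesh.
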(event `self.TrapActivator.OnComponentBeginOverlap`
  (params (OverlappedComponent :type "PrimitiveComponent Object Reference") (OtherActor :type "Actor Object Reference") (OtherComp :type "PrimitiveComponent Object Reference") (OtherBodyIndex :type Integer) (bFromSweep :type Boolean) (SweepResult :type "HitResult Structure (by ref)"))
  ;[0.5 0 0] If the landmine is activable than all activate landmine event
  (cast `/Game/FPSGame/Character/BP_Player` OtherActor)
  (if (`|EnumEquality` (`self.LandmineType`) "NewEnumerator1")
    (`self.ActivateLandmine`)))

(event `ActivateLandmine`
  ;[0.5 0 0] Make the landmine move upward and expload and damage actor
  (`/Engine/EditorBlueprintResources/StandardMacros.DoOnce` false
    (:`Completed`
      (bind (_direction _trap_activate) (`Timeline|LandmineTimeLine`)
        (:`Update`
          (`SceneComponent.K2_SetRelativeLocation` (`self.Cube`) (`KismetMathLibrary.VLerp` (0.0 0.0 -50.0) (0.0 0.0 0.0) _trap_activate) false true))))))

(event `self.Box.OnComponentBeginOverlap`
  (params (OverlappedComponent :type "PrimitiveComponent Object Reference") (OtherActor :type "Actor Object Reference") (OtherComp :type "PrimitiveComponent Object Reference") (OtherBodyIndex :type Integer) (bFromSweep :type Boolean) (SweepResult :type "HitResult Structure (by ref)"))
  ;[0.5 0 0] When the player overlap with the landmine damage the player
  (bind _asbp_player (cast `/Game/FPSGame/Character/BP_Player` OtherActor))
  (`GameplayStatics.SpawnEmitterAtLocation` "/Game/MilitaryWeapSilver/FX/P_Grenade_Explosion_01.P_Grenade_Explosion_01")
  (`GameplayStatics.PlaySoundAtLocation` "/Game/MilitaryWeapSilver/Sound/GrenadeLauncher/Wavs/GrenadeLauncher_Explosion05.GrenadeLauncher_Explosion05" (0.0 0.0 0.0) (struct) 1.0 1.0 0.0 null null null)
  (`GameplayStatics.ApplyDamage` _asbp_player (`self.Damage`) null self "/Engine/EngineDamageTypes/DmgTypeBP_Environmental.DmgTypeBP_Environmental_C")
  (`ActorComponent.K2_DestroyComponent` (`self.Box`))
  (`ActorComponent.K2_DestroyComponent` (`self.Cube`)))

(fn `UserConstructionScript`
  ;[0.5 0 0] Switch on the type of landmine
  (switch `/Game/FPSGame/Enemies/Explosives/ENUM_LandmineType` (`self.LandmineType`)
    (:`NewEnumerator0`
      (`SceneComponent.K2_SetRelativeLocation` (`self.Cube`) (0.0 0.0 0.0) false false))
    (:`NewEnumerator1`
      (`SceneComponent.K2_SetRelativeLocation` (`self.Cube`) (0.0 0.0 -50.0) false true))))