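; Parent Blueprint for enemy guns, providing hitscan firing for a gun whose parent actor is a BP_Enemy.
; StartShooting and StopShooting only toggle IsFiring.
; FireBullet line-traces from the enemy's camera and, on a blocking hit, spawns a bullet-hole decal, plays a looping fire animation and damages damageable actors.
; A separate HitPhysicsObjects function pushes physics-simulating components along the shot direction, though nothing here calls it or FireBullet.
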(event `StartShooting`
  (set `self.isFiring` true))

(event `StopShooting`
  (set `self.isFiring` false))

(fn `FireBullet`
  (locals (gunDirection :type "Vector Structure" :default (0.0 0.0 0.0)))
  (bind _asbp_enemy (cast `/Game/FPSGame/Enemies/BP_enemy` (`self.GetParentActor`)))
  (bind _camera (`/Game/FPSGame/Enemies/BP_enemy.Camera` _asbp_enemy))
  (bind _returnvalue (`KismetMathLibrary.GetForwardVector` (`SceneComponent.K2_GetComponentRotation` _camera)))
  (set `local.gunDirection` _returnvalue)
  (bind _returnvalue_2 (`SceneComponent.K2_GetComponentLocation` _camera))
  (bind _outhit (`KismetSystemLibrary.LineTraceSingle` _returnvalue_2 (+ _returnvalue_2 (* _returnvalue 3000.0)) "TraceTypeQuery1"))
  (bind (_bblockinghit _binitialoverlap _time _distance _location _impactpoint _normal _impactnormal _physmat _hitactor) (`GameplayStatics.BreakHitResult` _outhit))
  (if _bblockinghit
    (`GameplayStatics.SpawnDecalAtLocation` "/Game/FPSGame/Enemies/EnemyGuns/M_BulletHoleDecal.M_BulletHoleDecal" (10.0 10.0 10.0) _location (`KismetMathLibrary.MakeRotFromX` _normal) 5.0)
    (`SkeletalMeshComponent.PlayAnimation` (`self.Guns`) "/Game/MilitaryWeapSilver/Weapons/Animations/Fire_Rifle_W.Fire_Rifle_W" true)
    (if (`Actor.bCanBeDamaged` _hitactor)
      (`GameplayStatics.ApplyDamage` _hitactor 0.02))))

(fn `HitPhysicsObjects`
  (params (isHitting :type Boolean) (HitComponent :type "SceneComponent Object Reference") (Location :type "Vector Structure") (ImpulseObject :type "PrimitiveComponent Object Reference") (GunDirection :type "Vector Structure"))
  (if isHitting
    (if (`SceneComponent.IsSimulatingPhysics` HitComponent "None")
      (`PrimitiveComponent.AddImpulseAtLocation` ImpulseObject (* (`local.gunDirection`) 200000.0) Location "None"))))

(fn `UserConstructionScript`)