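; BP_enemy is the FPS enemy character: it fires a child-actor gun on start/stop events and takes bullet and explosive damage.
; Bullet damage scales by the hit physical material's DestructibleDamageThresholdScale, explosive damage by linear distance falloff.
; Hits spawn damage-number widgets, with hit markers for bullets only.
; Death triggers impulse-driven ragdoll, removes capsule and gun, and decrements the GameMode's enemy count, showing the win screen at zero.
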(event `self.ReceiveBeginPlay`
  ;[0.5 0 0] Reference to player
  (bind _asbp_player (cast `/Game/FPSGame/Character/BP_Player` (`GameplayStatics.GetPlayerCharacter` 0)))
  (set `self.Player` _asbp_player)
  ;[0.5 0 0] Reference to Anim Instance
  (bind _asue4asp_hero_tpp_anim_blueprint (cast `/Game/AnimStarterPack/UE4ASP_HeroTPP_AnimBlueprint` (`SkeletalMeshComponent.GetAnimInstance` (`self.Mesh`))))
  (set `self.AnimInstance` _asue4asp_hero_tpp_anim_blueprint)
  ;[0.5 0 0] Reference to BP_Gun
  (bind _asbp_gun__auto (cast `/Game/FPSGame/Enemies/EnemyGuns/BP_Gun-Auto` (`ChildActorComponent.ChildActor` (`self.Gun`))))
  (set `self.CurrentGun` _asbp_gun__auto)
  ;[0.5 0 0] Reference to game mode
  (bind _asbp_game_mode_base (cast `/Game/FPSGame/Blueprints/BP_GameModeBase` (`GameplayStatics.GetGameMode`)))
  (set `/Game/FPSGame/Blueprints/BP_GameModeBase.TotalEnemiesAlive` (+ (`/Game/FPSGame/Blueprints/BP_GameModeBase.TotalEnemiesAlive` _asbp_game_mode_base) 1) _asbp_game_mode_base))

(event `/Game/FPSGame/Interfaces/BPI_TakeDamage.EnemyTakeDamage`
  (params (WeaponStats :type "/Game/FPSGame/Data/S_WeaponStats Structure") (HitResults :type "HitResult Structure"))
  (bind (_bblockinghit _binitialoverlap _time _distance _location _impactpoint _normal _impactnormal _physmat _hitactor _hitcomponent _hitbonename) (`GameplayStatics.BreakHitResult` HitResults))
  ;[0.5 0 0] Enemy taking damage
  (if (not (`self.isDead?`))
    (bind _calculateddamage (`self.CalculateDamage` (`.Damage_3_BB6A0C124088AE922AA13A8A860532DF` (break `/Game/FPSGame/Data/S_WeaponStats` WeaponStats)) HitResults))
    (bind _isdead_ (`self.HealthUpdate` _calculateddamage))
    (bind _output_get (set `self.isDead?` _isdead_))
    (if _output_get
      (`self.EnemyDeath` _impactnormal _hitbonename))
    (`self.DamageNumbers` _calculateddamage _impactnormal (`|EnumEquality` (`PhysicalMaterial.SurfaceType` _physmat) "SurfaceType1"))
    (`/Engine/EditorBlueprintResources/StandardMacros.IsValid` (`self.HitMarkerRefer`)
      (:`Is Valid`
        (`Widget.RemoveFromParent` (`self.HitMarkerRefer`)) ; Removes previous marker if another hit occurs before the first
      )
      (:`Is Not Valid`
        _))
    ;[0.5 0 0] Add hit markers
    (bind _returnvalue (`|CreateWidget` "/Game/FPSGame/UI/W_HitMarkers.W_HitMarkers_C" null (`self.isDead?`)))
    (bind _output_get_2 (set `self.HitMarkerRefer` _returnvalue))
    (`UserWidget.AddToViewport` _output_get_2 0)))

(event `self.DamageNumbers`
  (params (Damage :type "Float (single-precision)") (ImpactLocation :type "Vector Structure") (`isHeadshot?` :type Boolean))
  (bind (_x _y) (`KismetMathLibrary.BreakVector2D` (`WidgetLayoutLibrary.ProjectWorldLocationToWidgetPosition` (`GameplayStatics.GetPlayerController` 0) ImpactLocation)))
  ;[0.5 0 0] Enemy taking damage and displaying the damage numbers
  (bind _returnvalue (`|CreateWidget` "/Game/FPSGame/UI/W_DamageNumbers.W_DamageNumbers_C" null Damage `isHeadshot?`))
  (`Widget.SetRenderTranslation` (`/Game/FPSGame/UI/W_DamageNumbers.SizeBox_57` _returnvalue) (`KismetMathLibrary.MakeVector2D` (+ (+ _x -100.0) (`KismetMathLibrary.RandomFloatInRange` -25.0 150.0)) (+ (+ _y -100.0) (`KismetMathLibrary.RandomFloatInRange` 0.0 50.0))))
  (`UserWidget.AddToViewport` _returnvalue 0))

(event `/Game/FPSGame/Interfaces/BPI_TakeDamage.TakeRadiusDamage`
  (params (HitResult :type "HitResult Structure") (WeaponStats :type "/Game/FPSGame/Data/S_WeaponStats Structure"))
  (bind (_damage _impactradius) (break `/Game/FPSGame/Data/S_WeaponStats` WeaponStats))
  (bind (_bblockinghit _binitialoverlap _time _distance _location _impactpoint _normal _impactnormal _physmat _hitactor _hitcomponent _hitbonename) (`GameplayStatics.BreakHitResult` HitResult))
  ;[0.5 0 0] Enemy takes explosion damage
  (if (not (`self.isDead?`))
    (bind _radiusdamageapplied (`self.CalculateRadiusDamage` _damage _impactradius _impactpoint))
    (bind _isdead_ (`self.HealthUpdate` _radiusdamageapplied))
    (if _isdead_
      (`self.EnemyDeath` _impactpoint _hitbonename))
    (`self.DamageNumbers` _radiusdamageapplied _impactpoint)))

(event `StartShooting`
  ;[0.5 0 0] Enemy AI start and stop shooting the player
  (if (not (`self.isDead?`))
    (`/Game/FPSGame/Enemies/EnemyGuns/BP_Gun-Parent.StartShooting` (`self.CurrentGun`))))

(event `StopShooting`
  ;[0.5 0 0] Enemy AI start and stop shooting the player
  (if (not (`self.isDead?`))
    (`/Game/FPSGame/Enemies/EnemyGuns/BP_Gun-Parent.StopShooting` (`self.CurrentGun`))))

(fn `CalculateDamage`
  (params (Damage :type "Float (double-precision)") (HitResult :type "HitResult Structure"))
  (returns (CalculatedDamage :type "Float (double-precision)"))
  (locals (LocalDamage :type "Float (double-precision)"))
  (set `local.LocalDamage` Damage)
  (return (* (`local.LocalDamage`) (`PhysicalMaterial.DestructibleDamageThresholdScale` (`.PhysMat` (`GameplayStatics.BreakHitResult` HitResult))))))

(fn `CalculateRadiusDamage`
  (params (Damage :type "Float (double-precision)") (ImpactRadius :type "Float (double-precision)") (ImpactPoint :type "Vector Structure"))
  (returns (RadiusDamageApplied :type "Float (double-precision)"))
  (set `self.Local Damage` Damage)
  (return (`KismetMathLibrary.FClamp` (* (- 1.0 (/ (`KismetMathLibrary.VSize` (- ImpactPoint (`self.K2_GetActorLocation`))) ImpactRadius)) (`self.Local Damage`)) 0.0 (`self.Local Damage`))))

(fn `EnemyDeath`
  (params (HitLocation :type "Vector Structure") (BoneName :type Name))
  (bind _returnvalue (`GameplayStatics.GetPlayerController` 0))
  (bind _player (`self.Player`))
  (`|ExecutionSequence`
    (:`then_0`
      ;[0.5 0 0] Enabling ragdoll physics
      (`PrimitiveComponent.SetSimulatePhysics` (`self.Mesh`) true))
    (:`then_1`
      (`GameplayStatics.PlaySound2D` "/Game/FPSGame/Sounds/A_EnemyDefeat.A_EnemyDefeat" 1.0 1.0 0.0 null null))
    (:`then_2`
      (`PrimitiveComponent.AddImpulseAtLocation` (`self.Mesh`) (* (`KismetMathLibrary.GetDirectionUnitVector` (`self.K2_GetActorLocation` _player) (`self.K2_GetActorLocation`)) (`/Game/FPSGame/Weapons/BP_WeaponBase.KillImpulse` (`/Game/FPSGame/Character/BP_Player.CurrentWeapon` _player))) HitLocation BoneName)
      ;[0.5 0 0] Destroying enemy and his gun on death
      (`ActorComponent.K2_DestroyComponent` (`self.CapsuleComponent`))
      (set `self.isDead?` true)
      (`ActorComponent.K2_DestroyComponent` (`self.Gun`))
      ;[0.5 0 0] Decrementing the enemies alive in the level on death
      (bind _asbp_game_mode_base (cast `/Game/FPSGame/Blueprints/BP_GameModeBase` (`GameplayStatics.GetGameMode`)))
      (bind _totalenemiesalive (`/Game/FPSGame/Blueprints/BP_GameModeBase.TotalEnemiesAlive` _asbp_game_mode_base))
      (set `/Game/FPSGame/Blueprints/BP_GameModeBase.TotalEnemiesAlive` (- _totalenemiesalive 1) _asbp_game_mode_base)
      ;[0.5 0 0] Checks if all the enemies are dead and display the game win screen
      (if (== _totalenemiesalive 0)
        (bind _returnvalue_2 (`|CreateWidget` "/Game/FPSGame/UI/W_GameWon.W_GameWon_C"))
        (`UserWidget.AddToViewport` _returnvalue_2 0)
        (`WidgetBlueprintLibrary.SetInputMode_UIOnlyEx` _returnvalue null)
        (set `PlayerController.bShowMouseCursor` true _returnvalue)))))

(fn `HealthUpdate`
  (params (DamageApplied :type "Float (double-precision)"))
  (returns (`isDead?` :type Boolean))
  (locals (`LocalisDead?` :type Boolean))
  (`|ExecutionSequence`
    (:`then_0`
      (if (>= DamageApplied (`self.CurrentHealth`))
        (set `local.LocalisDead?` true)
        (set `self.CurrentHealth` 0.0)
        (else
          (set `self.CurrentHealth` (- (`self.CurrentHealth`) DamageApplied)))))
    (:`then_1`
      (return (`local.LocalisDead?`)))))

(fn `UserConstructionScript`)