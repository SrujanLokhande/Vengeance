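; Base impact effect actor that plays surface-specific particles, sound and a decal at a hit point when it begins play.
; It reads the physical material's surface type from HitResults to choose between stone, body and water effects, with body-part surfaces sharing body effects and stone as default.
; The decal, distinct only for water, aligns to the hit normal with random roll and attaches to the hit component and bone.
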(event `self.ReceiveBeginPlay`
  (bind _stonefx (`self.StoneFX`))
  (bind _stonesfx (`self.StoneSFX`))
  (bind _bodysfx (`self.BodySFX`))
  (bind _impactdecail (`self.ImpactDecail`))
  (bind _decailsize (`self.DecailSize`))
  (bind _bodyfx (`self.BodyFX`))
  (bind (_bblockinghit _binitialoverlap _time _distance _location _impactpoint _normal _impactnormal _physmat) (`GameplayStatics.BreakHitResult` (`self.HitResults`)))
  (bind (_bblockinghit_2 _binitialoverlap_2 _time_2 _distance_2 _location_2 _impactpoint_2 _normal_2 _impactnormal_2 _physmat_2) (`GameplayStatics.BreakHitResult` (`self.HitResults`)))
  (bind (_bblockinghit_3 _binitialoverlap_3 _time_3 _distance_3 _location_3 _impactpoint_3 _normal_3 _impactnormal_3 _physmat_3 _hitactor _hitcomponent _hitbonename) (`GameplayStatics.BreakHitResult` (`self.HitResults`)))
  (`|ExecutionSequence`
    (:`then_0`
      (if _bblockinghit_2
        ;[0.5 0 0] Particle effects for different surface types
        (`GameplayStatics.SpawnEmitterAtLocation` (select `EPhysicalSurface` (`PhysicalMaterial.SurfaceType` _physmat_2) :`SurfaceType_Default` _stonefx :`SurfaceType1` _bodyfx :`SurfaceType2` _bodyfx :`SurfaceType3` _bodyfx :`SurfaceType4` _bodyfx :`SurfaceType5` _bodyfx :`SurfaceType6` _bodyfx :`SurfaceType7` _stonefx :`SurfaceType8` (`self.WaterFX`)) _impactpoint_2)))
    (:`then_1`
      (if _bblockinghit
        ;[0.5 0 0] Sound effects for different surface types
        (`GameplayStatics.PlaySoundAtLocation` (select `EPhysicalSurface` (`PhysicalMaterial.SurfaceType` _physmat) :`SurfaceType_Default` _stonesfx :`SurfaceType1` _bodysfx :`SurfaceType2` _bodysfx :`SurfaceType3` _bodysfx :`SurfaceType4` _bodysfx :`SurfaceType5` _bodysfx :`SurfaceType6` _bodysfx :`SurfaceType7` _stonesfx :`SurfaceType8` (`self.WaterSFX`) :!type "SoundBase Object Reference") _impactpoint (struct) 1.0 1.0 0.0 null null null)))
    (:`then_2`
      ;[0.5 0 0] Randomizes decail rotation
      (set `self.DecailRotation` (`KismetMathLibrary.MakeRotator` (`KismetMathLibrary.RandomFloatInRange` -180.0 180.0) (.pitch (`KismetMathLibrary.Conv_VectorToRotator` (`.Normal` (`GameplayStatics.BreakHitResult` (`self.HitResults`))))) (.yaw (`KismetMathLibrary.Conv_VectorToRotator` (`.Normal` (`GameplayStatics.BreakHitResult` (`self.HitResults`))))))))
    (:`then_3`
      (if _bblockinghit_3
        ;[0.5 0 0] Impact Details for different surface types
        (`GameplayStatics.SpawnDecalAttached` (select `EPhysicalSurface` (`PhysicalMaterial.SurfaceType` _physmat_3) :`SurfaceType_Default` _impactdecail :`SurfaceType1` _impactdecail :`SurfaceType2` _impactdecail :`SurfaceType3` _impactdecail :`SurfaceType4` _impactdecail :`SurfaceType5` _impactdecail :`SurfaceType6` _impactdecail :`SurfaceType7` _impactdecail :`SurfaceType8` (`self.WaterImpactDecail`) :!type "MaterialInterface Object Reference") (`KismetMathLibrary.MakeVector` _decailsize _decailsize _decailsize) _hitcomponent _hitbonename _impactpoint_3 (`self.DecailRotation`) "KeepWorldPosition" (`self.DecailLifeSpan`))))))

(fn `UserConstructionScript`)