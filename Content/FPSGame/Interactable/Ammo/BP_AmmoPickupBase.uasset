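; Base ammo pickup actor that gives ammo to the player's currently held weapon when picked up.
; On BeginPlay it caches the player character as BP_Player.
; PickupAmmo passes its AmmoType to the current weapon's AmmoPickup, which decides whether the ammo is taken.
; Only on success does it play a pickup sound and destroy itself.
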(event `self.ReceiveBeginPlay`
  ;[0.5 0 0] Reference to player
  (bind _asbp_player (cast `/Game/FPSGame/Character/BP_Player` (`GameplayStatics.GetPlayerCharacter` 0)))
  (set `self.Player` _asbp_player))

(event `PickupAmmo`
  ;[0.5 0 0] Add ammo amount (in weapon base)
  (bind _success (`/Game/FPSGame/Weapons/BP_WeaponBase.AmmoPickup` (`/Game/FPSGame/Character/BP_Player.CurrentWeapon` (`self.Player`)) (`self.AmmoType`)))
  (if _success
    (`GameplayStatics.PlaySound2D` (`self.PickupAmmoSound`) 1.0 1.0 0.0 null null)
    (`self.K2_DestroyActor`)))

(fn `UserConstructionScript`)