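; Base weapon pickup that bobs in the world and hands its weapon to the player on interaction.
; BeginPlay caches player 0 as BP_Player, and InteractedWithWeapon passes WeapontoSpawn to that player's WeaponPickup.
; A DoOnce after that call guards the pickup sound and the actor's destruction.
; The hover comes from the Bob timeline, played from Tick, adding its HoverAnim value as a local offset.
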(event `self.ReceiveBeginPlay`
  ;[0.5 0 0] Reference to player
  (bind _asbp_player (cast `/Game/FPSGame/Character/BP_Player` (`GameplayStatics.GetPlayerCharacter` 0)))
  (set `self.Player` _asbp_player))

(event `InteractedWithWeapon`
  ;[0.5 0 0] Runs event in BP Player
  (`/Game/FPSGame/Character/BP_Player.WeaponPickup` (`self.Player`) (`self.WeapontoSpawn`))
  (`/Engine/EditorBlueprintResources/StandardMacros.DoOnce` false
    (:`Completed`
      (`GameplayStatics.PlaySound2D` (`self.PickupSound`) 1.0 1.0 0.0 null null)
      (`self.K2_DestroyActor`))))

(event `self.ReceiveTick`
  (params (DeltaSeconds :type "Float (single-precision)"))
  ;[0.5 0 0] Hover Weapons up and down
  (bind (_direction _hoveranim) (`Timeline|Bob`)
    (:`Update`
      (`self.K2_AddActorLocalOffset` _hoveranim))))

(fn `UserConstructionScript`)