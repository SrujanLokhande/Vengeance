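; Base projectile Blueprint that applies weapon damage when its ProjectileMovement stops.
; Depending on IsDealingRadiusDamage, it sends a damage message to the hit actor or runs a sphere overlap at the impact point.
; The radius path messages each overlapped actor, ignoring the player's current weapon, and spawns BP_ExplosionImpulse.
; Both paths then spawn the ImpactEffect actor and set a short lifespan to destroy the projectile.
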(event `self.ReceiveBeginPlay`
  ;[0.5 0 0] Reference to player
  (bind _asbp_player (cast `/Game/FPSGame/Character/BP_Player` (`GameplayStatics.GetPlayerCharacter` 0)))
  (set `self.Player` _asbp_player))

(event `self.ProjectileMovement.OnProjectileStop`
  (params (ImpactResult :type "HitResult Structure (by ref)"))
  (`self.StopProjectile` ImpactResult))

(fn `ExplodeProjectile`
  (params (HitResult :type "HitResult Structure"))
  (bind (_bblockinghit _binitialoverlap _time _distance _location _impactpoint) (`GameplayStatics.BreakHitResult` HitResult))
  (`|ExecutionSequence`
    (:`then_0`
      (bind _outactors (`KismetSystemLibrary.SphereOverlapActors` _impactpoint (`.ImpactRadius_5_C2A1072C46D35F0B7B4EFB86F85D2817` (break `/Game/FPSGame/Data/S_WeaponStats` (`self.WeaponStats`))) (`|MakeArray` "ObjectTypeQuery2" "ObjectTypeQuery3" :!type "EObjectTypeQuery Enum") null (`|MakeArray` (`/Game/FPSGame/Character/BP_Player.CurrentWeapon` (`self.Player`)) :!type "Actor Object Reference")))
      (for _array_element _outactors
        (message `/Game/FPSGame/Interfaces/BPI_TakeDamage.TakeRadiusDamage` _array_element HitResult (`self.WeaponStats`))))
    (:`then_1`
      (`|SpawnActorFromClass` "/Game/FPSGame/Projectiles/BP_ExplosionImpulse.BP_ExplosionImpulse_C" (`KismetMathLibrary.MakeTransform` _impactpoint) "AlwaysSpawn" "OverrideRootScale" null null))))

(fn `StopProjectile`
  (params (HitResult :type "HitResult Structure"))
  (bind _projectilemesh (`self.ProjectileMesh`))
  (`|ExecutionSequence`
    (:`then_0`
      (if (`self.isDealingRadiusDamage?`)
        (`self.ExplodeProjectile` HitResult)
        (else
          (message `/Game/FPSGame/Interfaces/BPI_TakeDamage.EnemyTakeDamage` (`.HitActor` (`GameplayStatics.BreakHitResult` HitResult)) (`self.WeaponStats`) HitResult))))
    (:`then_1`
      ;[0.5 0 0] Removes mesh, Spawns Impact effect, destroys actor
      (`SceneComponent.SetHiddenInGame` _projectilemesh false false)
      (`|SpawnActorFromClass` (`self.ImpactEffect`) (`SceneComponent.K2_GetComponentToWorld` _projectilemesh) "AlwaysSpawn" "OverrideRootScale" null HitResult null)
      (`self.SetLifeSpan` 0.1))))

(fn `UserConstructionScript`)