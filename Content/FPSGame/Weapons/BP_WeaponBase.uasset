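; BP_WeaponBase is the base FPS weapon, handling firing, ammo, reloading and aim state for BP_Player.
; StartShooting spends a round, auto-reloads when empty, then fires camera line traces (multiple for shotguns, spread when not aiming) or spawns muzzle-socket projectiles.
; Hits send WeaponStats to enemies and spawn impact effects, while a reversing timeline drives recoil.
; Helpers handle typed ammo pickups, reload math and fire-rate lockout; Tick updates the player's aim FOV.
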(event `self.ReceiveBeginPlay`
  ;[0.5 0 0] Reference to player
  (bind _asbp_player (cast `/Game/FPSGame/Character/BP_Player` (`GameplayStatics.GetPlayerCharacter` 0)))
  (bind _output_get (set `self.Player` _asbp_player))
  ;[0.5 0 0] Binds aiming bool to ADS input Action on BP_Player
  (add `/Game/FPSGame/Character/BP_Player.AimEnter` _output_get (delegate `WeaponAimEnter`))
  (add `/Game/FPSGame/Character/BP_Player.AimExit` _output_get (delegate `WeaponAimExit`)))

(event `WeaponAimEnter`
  ;[0.5 0 0] Binds aiming bool to ADS input Action on BP_Player
  (set `self.isAimingWeapon?` true))

(event `WeaponAimExit`
  ;[0.5 0 0] Binds aiming bool to ADS input Action on BP_Player
  (set `self.isAimingWeapon?` false))

(event `AutoReloadOnEmpty`
  ;[0.5 0 0] Automatically reloads
  (if (`|EnumEquality` (`self.Weapon`) "NewEnumerator3")
    (`KismetSystemLibrary.Delay` 0.3)
    (`/Game/FPSGame/Character/BP_Player.Reload` (`self.Player`))
    (`self.WeaponAimExit`)
    (else
      (`/Game/FPSGame/Character/BP_Player.Reload` (`self.Player`)))))

(event `StartRecoil`
  (bind _returnvalue (`GameplayStatics.GetPlayerCharacter` 0))
  ;[0.5 0 0] Adds Recoil effect to weapoons
  (bind (_direction _alpha) (`Timeline|Recoil` :!via `PlayFromStart` :!label _label)
    (:`Update`
      (switch `ETimelineDirection` _direction
        (:`Forward`
          (bind _returnvalue_2 (`KismetMathLibrary.Lerp` 0.0 (`self.WeaponKick`) _alpha))
          (`Pawn.AddControllerPitchInput` _returnvalue _returnvalue_2)
          (`Pawn.AddControllerYawInput` (`GameplayStatics.GetPlayerCharacter` 0) (`KismetMathLibrary.RandomFloatInRange` -0.15 0.15)))
        (:`Backward`
          (`Pawn.AddControllerPitchInput` _returnvalue (* _returnvalue_2 -1.0)))))
    (:`Finished`
      (`self.ReverseRecoil`)
      (`KismetSystemLibrary.RetriggerableDelay` 0.05)
      (`self.StopRecoil`))))

(event `StopRecoil`
  ;[0.5 0 0] Adds Recoil effect to weapoons
  (goto _label :!via `Stop`))

(event `ReverseRecoil`
  ;[0.5 0 0] Adds Recoil effect to weapoons
  (goto _label :!via `Reverse`))

(event `FireRateCalculate`
  ;[0.5 0 0] FireRate for non-automatic weapons
  (set `/Game/FPSGame/Character/BP_Player.isWeaponFireLoading?` true (`self.Player`))
  (`KismetSystemLibrary.Delay` (`self.FireRate`))
  (set `/Game/FPSGame/Character/BP_Player.isWeaponFireLoading?` false (`self.Player`)))

(event `self.ReceiveTick`
  (params (DeltaSeconds :type "Float (single-precision)"))
  (`/Game/FPSGame/Character/BP_Player.AimFieldOfView` (`self.Player`)))

(fn `AddDamage`
  (params (HitResult :type "HitResult Structure"))
  ;[0.5 0 0] Passes info through weapon to enemy taking damage
  (message `/Game/FPSGame/Interfaces/BPI_TakeDamage.EnemyTakeDamage` (`.HitActor` (`GameplayStatics.BreakHitResult` HitResult)) (`self.WeaponStats`) HitResult))

(fn `AmmoPickup`
  (params (AmmoType :type "/Game/FPSGame/Data/E_AmmoType Enum" :default "NewEnumerator0"))
  (returns (Success :type Boolean))
  (switch `/Game/FPSGame/Data/E_AmmoType` AmmoType
    (:`NewEnumerator0`
      ;[0.5 0 0] Adds ammo after picking up pistol ammo
      (if (`|EnumEquality` (`self.Weapon`) "NewEnumerator0")
        (set `self.CurrentTotalAmmo` (+ (`self.PistolPickupAmount`) (`self.CurrentTotalAmmo`)))
        (return true)
        (else
          (return false))))
    (:`NewEnumerator1`
      ;[0.5 0 0] Adds ammo after picking up autorifle ammo
      (if (`|EnumEquality` (`self.Weapon`) "NewEnumerator1")
        (set `self.CurrentTotalAmmo` (+ (`self.AutoRiflePickupAmount`) (`self.CurrentTotalAmmo`)))
        (return true)
        (else
          (return false))))
    (:`NewEnumerator2`
      ;[0.5 0 0] Adds ammo after picking up shotgun ammo
      (if (`|EnumEquality` (`self.Weapon`) "NewEnumerator2")
        (set `self.CurrentTotalAmmo` (+ (`self.ShotgunPickupAmpunt`) (`self.CurrentTotalAmmo`)))
        (return true)
        (else
          (return false))))
    (:`NewEnumerator3`
      ;[0.5 0 0] Adds ammo after picking up SniperRifle ammo
      (if (`|EnumEquality` (`self.Weapon`) "NewEnumerator3")
        (set `self.CurrentTotalAmmo` (+ (`self.SniperRiflePickupAmount`) (`self.CurrentTotalAmmo`)))
        (return true)
        (else
          (return false))))
    (:`NewEnumerator4`
      ;[0.5 0 0] Adds ammo after picking up Grenadelauncher ammo
      (if (`|EnumEquality` (`self.Weapon`) "NewEnumerator4")
        (set `self.CurrentTotalAmmo` (+ (`self.GrenadeLauncherPickupAmount`) (`self.CurrentTotalAmmo`)))
        (return true)
        (else
          (return false))))
    (:`NewEnumerator5`
      ;[0.5 0 0] Adds ammo after picking up rocketlauncher ammo
      (if (`|EnumEquality` (`self.Weapon`) "NewEnumerator5")
        (set `self.CurrentTotalAmmo` (+ (`self.RocketLauncherPickupAmount`) (`self.CurrentTotalAmmo`)))
        (return true)
        (else
          (return false))))))

(fn `CalculateLineTrace`
  (params (CameraComponent :type "CameraComponent Object Reference"))
  (returns (HitResult :type "HitResult Structure"))
  (locals (LocalCamera :type "CameraComponent Object Reference") (LocalWeaponMesh :type "SceneComponent Object Reference") (LocalWeaponSocket :type Name))
  (bind _bulletspread (`self.BulletSpread`))
  (bind (_returnvalue_location _returnvalue_rotation _returnvalue_scale) (`KismetMathLibrary.BreakTransform` (`SceneComponent.K2_GetComponentToWorld` (`local.LocalCamera`))))
  (bind _returnvalue (* _bulletspread -1.0))
  (bind _returnvalue_2 (+ _returnvalue_scale (* (`KismetMathLibrary.GetForwardVector` _returnvalue_rotation) 10000.0)))
  ;[1 0 0] Calculates the line trace
  (`|ExecutionSequence`
    (:`then_0`
      (set `local.LocalCamera` CameraComponent))
    (:`then_1`
      (bind _outhit (`KismetSystemLibrary.LineTraceSingleForObjects` _returnvalue_location (select `bool` (`/Game/FPSGame/Character/BP_Player.IsAiming?` (`self.Player`)) :`false` (`KismetMathLibrary.MakeVector` (+ (.x _returnvalue_2) (`KismetMathLibrary.RandomFloatInRange` _returnvalue _bulletspread)) (+ (.y _returnvalue_2) (`KismetMathLibrary.RandomFloatInRange` _returnvalue _bulletspread)) (+ (.z _returnvalue_2) (`KismetMathLibrary.RandomFloatInRange` _returnvalue _bulletspread))) :`true` _returnvalue_2) (`|MakeArray` "ObjectTypeQuery1" "ObjectTypeQuery2" :!type "EObjectTypeQuery Enum") false (`|MakeArray` (`GameplayStatics.GetPlayerCharacter` 0) :!type "Actor Object Reference"))))
    (:`then_2`
      (return _outhit))))

(fn `CalculateProjectile`
  (params (CameraComponent :type "CameraComponent Object Reference") (WeaponMesh :type "SceneComponent Object Reference") (WeaponSocket :type Name))
  (returns (ProjectileTransform :type "Transform Structure"))
  (locals (LocalCamera :type "CameraComponent Object Reference") (LocalWeaponMesh :type "SceneComponent Object Reference") (LocalWeaponSocket :type Name) (`Local WeaponMesh` :type "SceneComponent Object Reference"))
  ;[1 0 0] Calculates the projectile
  (`|ExecutionSequence`
    (:`then_0`
      (set `local.LocalCamera` CameraComponent)
      (set `local.Local WeaponMesh` WeaponMesh)
      (set `local.LocalWeaponSocket` WeaponSocket))
    (:`then_1`
      (set `self.ProjectileTransform` (`KismetMathLibrary.MakeTransform` (`SceneComponent.GetSocketLocation` (`local.Local WeaponMesh`) (`local.LocalWeaponSocket`)) (`Pawn.GetControlRotation` (cast `/Game/FPSGame/Character/BP_Player` (`ActorComponent.GetOwner` (`local.LocalCamera`)) :!pure true)))))
    (:`then_2`
      (return (`self.ProjectileTransform`)))))

(fn `DoWeHaveAmmo?`
  (returns (`HasAmmo?` :type Boolean))
  ;[0.5 0 0] Allows Shoot event to occur if player has ammo
  (return (> (`self.CurrentAmmo`) 0)))

(fn `isMagFull orEmpty?`
  (returns (ReturnValue :type Boolean))
  (if (== (`self.CurrentAmmo`) (`self.Magazine Size`))
    _
    (elif (== (`self.CurrentTotalAmmo`) 0)
      _
      (else
        ;[0.5 0 0] Enables reload if magazine is empty but ammo is left in reserve
        (bind _output_get (set `/Game/FPSGame/Character/BP_Player.CanReload?` true (`self.Player`)))
        (return _output_get))))
  ;[0.5 0 0] Disables reload if magazine is full or reserves are empty
  (bind _output_get_2 (set `/Game/FPSGame/Character/BP_Player.CanReload?` false (`self.Player`)))
  (return _output_get_2))

(fn `isThereAmmoLeft?`
  (returns (`isThereAmmoLeft?` :type Boolean))
  ;[0.5 0 0] Checks to see if there is ammo in reserves
  (return (> (`self.CurrentTotalAmmo`) 0)))

(fn `Reload Calculation`
  (bind _output_get (set `self.Bullet Difference` (- (`self.Magazine Size`) (`self.CurrentAmmo`))))
  (if (<= _output_get (`self.CurrentTotalAmmo`))
    ;[0.5 0 0] Runs when there is reserve ammo
    (set `self.CurrentAmmo` (`self.Magazine Size`))
    (set `self.CurrentTotalAmmo` (- (`self.CurrentTotalAmmo`) (`self.Bullet Difference`)))
    (else
      ;[0.5 0 0] Run when reserve amount is lower than ammo in magazine
      (set `self.CurrentAmmo` (+ (`self.CurrentAmmo`) (`self.CurrentTotalAmmo`)))
      (set `self.CurrentTotalAmmo` 0))))

(fn `ShotgunReloadPellets`
  (set `self.ReloadTime` (* (- (`self.Magazine Size`) (`self.CurrentAmmo`)) (`self.ReloadTime`))))

(fn `StartShooting`
  (params (FireType :type "/Game/FPSGame/Data/E_FireType Enum" :default "NewEnumerator0"))
  (`|ExecutionSequence`
    (:`then_0`
      ;[0.5 0 0] Subtracts 1 bullet when firing weapon
      (set `self.CurrentAmmo` (- (`self.CurrentAmmo`) 1))
      ;[0.5 0 0] Automatically Reloads when Mag runs out
      (if (<= (`self.CurrentAmmo`) 0)
        (`self.AutoReloadOnEmpty`)))
    (:`then_1`
      (switch `/Game/FPSGame/Data/E_FireType` FireType
        (:`NewEnumerator0`
          (if (`self.isShotgun?`)
            (for _ (range (`self.PelletCount`))
              ;[0.5 0 0] Draws line trace for HitScan Weapons
              (bind _hitresult (`self.CalculateLineTrace` (`/Game/FPSGame/Character/BP_Player.Camera` (`self.Player`)) :!label _label))
              (`self.AddDamage` _hitresult)
              ;[0.5 0 0] Spawns imapact effect at HitResult
              (`|SpawnActorFromClass` (`self.ImpactEffect`) (`KismetMathLibrary.MakeTransform` (`.ImpactPoint` (`GameplayStatics.BreakHitResult` _hitresult))) "Undefined" "OverrideRootScale" null _hitresult null)
              (`self.StartRecoil` :!label _label_2)
              (set `self.isFiring?` true))
            (else
              (goto _label))))
        (:`NewEnumerator1`
          ;[0.5 0 0] Spawns projectile
          (bind _projectiletransform (`self.CalculateProjectile` (`/Game/FPSGame/Character/BP_Player.Camera` (`self.Player`)) (`self.WeaponMesh`) "MuzzleFlash"))
          (`|SpawnActorFromClass` (`self.Projectile`) _projectiletransform "AlwaysSpawn" "OverrideRootScale" null (`self.WeaponStats`) null)
          (goto _label_2))))))

(fn `StopShooting`
  (set `self.isFiring?` false))

(fn `UserConstructionScript`)