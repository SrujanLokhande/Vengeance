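; Sniper rifle weapon Blueprint that extends a parent weapon with a fire animation and a scoped aiming view.
; Shooting runs the parent logic, plays the rifle mesh animation, then calls the fire-rate calculation.
; Entering aim on the current weapon creates a crosshair widget and hides the weapon mesh, player character and main HUD.
; Exiting aim removes the widget and restores all three.
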(event `self.StartShooting`
  (params (FireType :type "/Game/FPSGame/Data/E_FireType Enum" :default "NewEnumerator0"))
  (`parent.StartShooting` FireType)
  (`SkeletalMeshComponent.PlayAnimation` (`self.WeaponMesh`) "/Game/MilitaryWeapSilver/Weapons/Animations/Fire_SniperRifle_W.Fire_SniperRifle_W" false)
  (`self.FireRateCalculate`))

(event `self.WeaponAimEnter`
  (`parent.WeaponAimEnter`)
  (if (== (`/Game/FPSGame/Character/BP_Player.CurrentWeapon` (`self.Player`)) self)
    (bind _returnvalue (`|CreateWidget` "/Game/FPSGame/UI/W_SniperCrosshair.W_SniperCrosshair_C"))
    (if (not (`Widget.IsInViewport` _returnvalue))
      (`UserWidget.AddToViewport` _returnvalue 0)
      ;[0.5 0 0] Hides weapon, player and HUD while ADS Sniper
      (`SceneComponent.SetHiddenInGame` (`self.WeaponMesh`) true false)
      (`self.SetActorHiddenInGame` (`GameplayStatics.GetPlayerCharacter` 0) true)
      (`Widget.SetVisibility` (`/Game/FPSGame/Character/BP_Player.MainHUD` (`self.Player`)) "Collapsed"))))

(event `self.WeaponAimExit`
  (`parent.WeaponAimExit`)
  (`/Engine/EditorBlueprintResources/StandardMacros.IsValid` (stale `self.WeaponAimEnter` _returnvalue)
    (:`Is Valid`
      (`Widget.RemoveFromParent` (stale `self.WeaponAimEnter` _returnvalue))
      ;[0.5 0 0] Shows weapon, player and HUD while ADS Sniper
      (`SceneComponent.SetHiddenInGame` (`self.WeaponMesh`) false false)
      (`self.SetActorHiddenInGame` (`GameplayStatics.GetPlayerCharacter` 0) false)
      (`Widget.SetVisibility` (`/Game/FPSGame/Character/BP_Player.MainHUD` (`self.Player`)) "Visible"))))

(fn `UserConstructionScript`
  (`parent.UserConstructionScript`))