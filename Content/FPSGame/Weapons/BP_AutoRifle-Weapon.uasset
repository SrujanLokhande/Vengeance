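; Automatic rifle weapon Blueprint that fires continuously while shooting is held active.
; StartShooting fires immediately, then a looping timer at the fire rate repeats AutoRifleFire, which calls the parent weapon's shooting logic and plays the rifle mesh fire animation.
; When ammo runs out it stops shooting and triggers the player's reload; StopShooting clears the timer.
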(event `self.StartShooting`
  (params (FireType :type "/Game/FPSGame/Data/E_FireType Enum" :default "NewEnumerator0"))
  (set `self.isAutoRifleShooting?` true)
  (`self.AutoRifleFire`)
  (bind _returnvalue (`KismetSystemLibrary.K2_SetTimerDelegate` (delegate `AutoRifleFire`) (`self.AutoRifleFireRate`) true)))

(event `AutoRifleFire`
  (if (`self.isAutoRifleShooting?`)
    (`parent.StartShooting` (stale `self.StartShooting` FireType))
    (`SkeletalMeshComponent.PlayAnimation` (`self.WeaponMesh`) "/Game/MilitaryWeapSilver/Weapons/Animations/Fire_Rifle_W.Fire_Rifle_W" false)
    (if (<= (`self.CurrentAmmo`) 0)
      (`self.StopShooting`)
      (`/Game/FPSGame/Character/BP_Player.Reload` (`self.Player`)))))

(event `self.StopShooting`
  (`parent.StopShooting`)
  (set `self.isAutoRifleShooting?` false)
  (`KismetSystemLibrary.K2_ClearAndInvalidateTimerHandle` (stale `self.StartShooting` _returnvalue)))

(fn `UserConstructionScript`
  (`parent.UserConstructionScript`))