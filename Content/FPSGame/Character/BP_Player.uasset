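; First-person player character for the FPS game, handling movement, health, weapons and HUD, plus pause and game-over screens.
; A camera line trace triggers weapon and ammo pickups; spawned weapons attach to arm sockets in six key-selected slots, swapped by visibility.
; Firing and ammo logic delegate to the current weapon, while timelines drive reload arm motion and sprint stamina with exhaustion.
; Aiming, sprinting and reloading interrupt each other through state flags and adjust walk speed.
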(event `self.ReceiveBeginPlay`
  ;[0.5 0 0] Create MainHUD
  (bind _returnvalue (`|CreateWidget` "/Game/FPSGame/UI/W_MainHUD.W_MainHUD_C"))
  (bind _output_get (set `self.MainHUD` _returnvalue))
  (`UserWidget.AddToViewport` _output_get 0))

(event `WeaponPickup`
  (params (WeaponToSpawn :type "/Game/FPSGame/Weapons/BP_WeaponBase Class Reference"))
  ;[1 0.02983 0] Creates the weapon pickup
  (bind _returnweapon (`self.SpawnWeapon` WeaponToSpawn))
  (`self.EquipWeapon` _returnweapon))

(event `EquipWeapon`
  (params (Weapon :type "/Game/FPSGame/Weapons/BP_WeaponBase Object Reference"))
  ;[1 0.02983 0] Equips the picked weapon in player hand
  (if (not (`self.isSwitchingWeapon?`))
    (if (`self.isReloading?`)
      (set `self.isReloading?` true))
    (set `self.isSwitchingWeapon?` true)
    (`self.HideAndShowWeaponMesh` Weapon)
    (set `self.Loadout` "NewEnumerator1")
    (`/Game/FPSGame/UI/W_Crosshair.Crosshair update` (`/Game/FPSGame/UI/W_MainHUD.Crosshair` (`self.MainHUD`)))
    (`KismetSystemLibrary.Delay` 0.3) ; Allows time for weapon switch
    (set `self.isSwitchingWeapon?` false)
    (set `self.Can Shoot?` true) ; Cant shoot while shooting weapon
  ))

(event `Fire`
  (bind _currentweapon (`self.CurrentWeapon`))
  (bind _currentweapon_2 (`self.CurrentWeapon`))
  (if (`self.Can Shoot?`)
    (if (`/Game/FPSGame/Weapons/BP_WeaponBase.DoWeHaveAmmo?` _currentweapon_2)
      (`/Game/FPSGame/Weapons/BP_WeaponBase.StartShooting` _currentweapon (`/Game/FPSGame/Weapons/BP_WeaponBase.FireType` _currentweapon))
      (elif (`/Game/FPSGame/Weapons/BP_WeaponBase.isThereAmmoLeft?` _currentweapon_2)
        ;[0.5 0 0] Reloads weapon if there is reserve ammo
        (`self.Reload`)
        (else
          (`GameplayStatics.PlaySound2D` "/Game/ShooterGame/Sounds/Weapons/GrenadeLauncher/wav/sw_Wep_Launcher_Dryfire_01.sw_Wep_Launcher_Dryfire_01" 1.0 1.0 0.0 null null))))))

(event `Reload`
  (bind _currentweapon (`self.CurrentWeapon`))
  (if (`self.CanWeReload?`)
    (`|ExecutionSequence`
      (:`then_0`
        (set `self.isReloading?` true)
        (set `self.Can Shoot?` false)
        (set `self.IsAiming?` false)
        ;[0.5 0 0] Controls animations for reloading
        (bind (_direction _pulldown) (`Timeline|WeaponPullDown` :!via `PlayFromStart`)
          (:`Update`
            (if (`self.isReloading?`)
              (set `self.PullDownTimer` _pulldown)))
          (:`Finished`
            (`KismetSystemLibrary.Delay` (`/Game/FPSGame/Weapons/BP_WeaponBase.ReloadTime` (`self.CurrentWeapon`)))
            (bind (_direction_2 _pullup) (`Timeline|WeaponPullUp` :!via `PlayFromStart`)
              (:`Update`
                (if (`self.isReloading?`)
                  (set `self.PullDownTimer` _pullup)
                  (`/Engine/EditorBlueprintResources/StandardMacros.DoOnce` false :!label _label
                    (:`Completed`
                      (`GameplayStatics.PlaySound2D` (`/Game/FPSGame/Weapons/BP_WeaponBase.ReloadEndSound` (`self.CurrentWeapon`)) 1.0 1.0 0.0 null null)
                      (`KismetSystemLibrary.Delay` 1.0)
                      (goto _label :!via `Reset`)))))
              (:`Finished`
                (if (`self.isReloading?`)
                  (`/Game/FPSGame/Weapons/BP_WeaponBase.Reload Calculation` (`self.CurrentWeapon`))
                  (set `self.isReloading?` false)
                  (set `self.Can Shoot?` true)))))))
      (:`then_1`
        (if (not (`self.isSprinting?`))
          (set `CharacterMovementComponent.MaxWalkSpeed` (`self.Max Walk Speed`) (`self.CharacterMovement`))))
      (:`then_2`
        ;[1 0.02983 0] Plays sound
        (`GameplayStatics.PlaySound2D` (`/Game/FPSGame/Weapons/BP_WeaponBase.ReloadStartSound` (`self.CurrentWeapon`)) 1.0 1.0 0.0 null null)
        (if (`/Game/FPSGame/Weapons/BP_WeaponBase.isShotgun?` (`self.CurrentWeapon`))
          (`/Game/FPSGame/Weapons/BP_WeaponBase.ShotgunReloadPellets` _currentweapon)
          (`KismetSystemLibrary.Delay` (`/Game/FPSGame/Weapons/BP_WeaponBase.ReloadTime` _currentweapon))
          (set `/Game/FPSGame/Weapons/BP_WeaponBase.ReloadTime` 0.3 _currentweapon))))))

(event `self.ReceiveAnyDamage`
  (params (Damage :type "Float (single-precision)") (DamageType :type "DamageType Object Reference") (InstigatedBy :type "Controller Object Reference") (DamageCauser :type "Actor Object Reference"))
  ;[0.5 0 0] open the retry screen when player dies
  (bind _output_get (set `self.Health` (- (`self.Health`) Damage)))
  (if (<= _output_get 0.0)
    (`PrimitiveComponent.SetSimulatePhysics` (`self.PlayerArms`) true)
    (`ActorComponent.K2_DestroyComponent` (`self.CapsuleComponent`))
    (`KismetSystemLibrary.Delay` 0.1)
    (bind _returnvalue (`|CreateWidget` "/Game/FPSGame/UI/W_GameEnd.W_GameEnd_C"))
    (`UserWidget.AddToViewport` _returnvalue 0)
    (set `PlayerController.bShowMouseCursor` true (`GameplayStatics.GetPlayerController` 0))
    (`GameplayStatics.SetGamePaused` true)
    (else
      (`KismetSystemLibrary.Delay` 3.0)
      (set `self.Health` (+ (`self.Health`) 0.1)))))

(event `InputAction|PauseMenu`
  (params (Key :type "Key Structure"))
  (bind _returnvalue (`GameplayStatics.GetPlayerController` 0))
  ;[0.5 0 0] Pause Game on hitting escape
  (:`Pressed`
    (`WidgetBlueprintLibrary.SetInputMode_UIOnlyEx` _returnvalue null)
    (bind _returnvalue_2 (`|CreateWidget` "/Game/FPSGame/UI/W_PauseMenu.W_PauseMenu_C"))
    (`UserWidget.AddToViewport` _returnvalue_2 0)
    (set `PlayerController.bShowMouseCursor` true _returnvalue)
    (`GameplayStatics.SetGamePaused` true)))

(event `InputAxis|MoveForward`
  (params (AxisValue :type "Float (single-precision)"))
  ;[0.5 0 0] WASD Movement Import
  (`self.AddMovementInput` (`KismetMathLibrary.GetForwardVector` (`KismetMathLibrary.MakeRotator` 0.0 0.0 (.yaw (`self.GetControlRotation`)))) AxisValue))

(event `InputAxis|MoveRight`
  (params (AxisValue :type "Float (single-precision)"))
  ;[0.5 0 0] WASD Movement Import
  (`self.AddMovementInput` (`KismetMathLibrary.GetRightVector` (`KismetMathLibrary.MakeRotator` 0.0 0.0 (.yaw (`self.GetControlRotation`)))) AxisValue))

(event `InputAction|Jump`
  (params (Key :type "Key Structure"))
  ;[0.5 0 0] Jump Action
  (:`Pressed`
    (`self.Jump`))
  (:`Released`
    (`self.StopJumping`)))

(event `self.ReceiveTick`
  (params (DeltaSeconds :type "Float (single-precision)"))
  ;[0.5 0 0] Checks if W is released while sprinting
  (if (`self.HaveWeStoppedMoving`)
    (`self.MovementStopped`) ; Connected to timeline
  ))

(event `InputAction|Sprint`
  (params (Key :type "Key Structure"))
  ;[0.5 0 0] Sprint with regenrating stamina bar
  (:`Pressed`
    (if (not (`self.IsAiming?`))
      (if true
        (if (`self.AreWeExhausted?`)
          (`self.StartSprint`)
          (switch `/Game/FPSGame/Data/E_Loadout` (`self.Loadout`)
            (:`NewEnumerator0`
              (bind (_direction _staminaamount) (`Timeline|Stamina` :!label _label)
                (:`Update`
                  (bind _output_get (set `self.EnergyLevel` _staminaamount)))
                (:`Finished`
                  (if (== _output_get 0.0)
                    (`self.Exhausted`)))))
            (:`NewEnumerator1`
              (`/Game/FPSGame/Weapons/BP_WeaponBase.StopShooting` (`self.CurrentWeapon`))
              (goto _label)))))))
  (:`Released`
    (if (`self.IsShiftKeyDown?`)
      (`self.MovementStopped`))))

(event `MovementStopped`
  ;[0.5 0 0] Sprint with regenrating stamina bar
  (if (not (`self.isExhausted?`))
    (`|ExecutionSequence`
      (:`then_0`
        (`self.StopSprint`)
        (goto _label :!via `Stop`))
      (:`then_1`
        (`KismetSystemLibrary.Delay` (`self.StaminaRegainPause`))
        (goto _label :!via `Reverse`)))))

(event `Exhausted`
  ;[0.5 0 0] Sprint with regenrating stamina bar
  (set `self.isExhausted?` true)
  (`self.StopSprint`)
  (`KismetSystemLibrary.Delay` (`self.ExhaustedTimer`))
  (set `self.isExhausted?` false)
  (goto _label :!via `ReverseFromEnd`))

(event `Key|One`
  (params (Key :type "Key Structure"))
  (bind _weaponslot01 (`self.WeaponSlot01`))
  ;[0.5 0 0] Key binding to equip weapons after they are picked up
  (:`Pressed`
    (if (`self.Is1stSlotFilled?`)
      (if (not (== (`self.CurrentWeapon`) (`self.WeaponSlot01`)))
        (`self.EquipWeapon` _weaponslot01)
        (set `self.CurrentWeapon` _weaponslot01)
        (`/Game/FPSGame/UI/W_Crosshair.Crosshair update` (`/Game/FPSGame/UI/W_MainHUD.Crosshair` (`self.MainHUD`)) :!label _label)))))

(event `Key|Two`
  (params (Key :type "Key Structure"))
  (bind _weaponslot02 (`self.WeaponSlot02`))
  ;[0.5 0 0] Key binding to equip weapons after they are picked up
  (:`Pressed`
    (if (`self.Is2ndSlotFilled?`)
      (if (not (== (`self.CurrentWeapon`) (`self.WeaponSlot02`)))
        (`self.EquipWeapon` _weaponslot02)
        (set `self.CurrentWeapon` _weaponslot02)
        (goto _label)))))

(event `Key|Three`
  (params (Key :type "Key Structure"))
  (bind _weaponslot03 (`self.WeaponSlot03`))
  ;[0.5 0 0] Key binding to equip weapons after they are picked up
  (:`Pressed`
    (if (`self.Is3rdSlotFilled?`)
      (if (not (== (`self.CurrentWeapon`) (`self.WeaponSlot03`)))
        (`self.EquipWeapon` _weaponslot03)
        (set `self.CurrentWeapon` _weaponslot03)
        (goto _label)))))

(event `Key|Four`
  (params (Key :type "Key Structure"))
  (bind _weaponslot04 (`self.WeaponSlot04`))
  ;[0.5 0 0] Key binding to equip weapons after they are picked up
  (:`Pressed`
    (if (`self.Is4thSlotFilled?`)
      (if (not (== (`self.CurrentWeapon`) (`self.WeaponSlot04`)))
        (`self.EquipWeapon` _weaponslot04)
        (set `self.CurrentWeapon` _weaponslot04)
        (goto _label)))))

(event `Key|Five`
  (params (Key :type "Key Structure"))
  (bind _weaponslot05 (`self.WeaponSlot05`))
  ;[0.5 0 0] Key binding to equip weapons after they are picked up
  (:`Pressed`
    (if (`self.Is5thSlotFilled?`)
      (if (not (== (`self.CurrentWeapon`) (`self.WeaponSlot05`)))
        (`self.EquipWeapon` _weaponslot05)
        (set `self.CurrentWeapon` _weaponslot05)
        (goto _label)))))

(event `Key|Six`
  (params (Key :type "Key Structure"))
  (bind _weaponslot06 (`self.WeaponSlot06`))
  ;[0.5 0 0] Key binding to equip weapons after they are picked up
  (:`Pressed`
    (if (`self.Is6thSlotFilled?`)
      (if (not (== (`self.CurrentWeapon`) (`self.WeaponSlot06`)))
        (`self.EquipWeapon` _weaponslot06)
        (set `self.CurrentWeapon` _weaponslot06)
        (goto _label)))))

(event `InputAction|Interact`
  (params (Key :type "Key Structure"))
  (bind _camera (`self.Camera`))
  (bind _returnvalue (`SceneComponent.K2_GetComponentLocation` _camera))
  ;[0.5 0 0] Draws a line trace to check if we interact with ammo or weapon
  (:`Pressed`
    (bind (_outhit _returnvalue_2) (`KismetSystemLibrary.LineTraceSingle` _returnvalue (+ _returnvalue (* (`SceneComponent.GetForwardVector` _camera) 200.0)) "TraceTypeQuery1"))
    (if _returnvalue_2
      (`|ExecutionSequence`
        (:`then_0`
          (switch `/Game/FPSGame/Data/E_Loadout` (`self.Loadout`) ; Cant grab ammo without weapon
            (:`NewEnumerator1`
              (bind (_bblockinghit _binitialoverlap _time _distance _location _impactpoint _normal _impactnormal _physmat _hitactor) (`GameplayStatics.BreakHitResult` _outhit))
              (bind _asbp_ammo_pickup_base (cast `/Game/FPSGame/Interactable/Ammo/BP_AmmoPickupBase` _hitactor))
              (`/Game/FPSGame/Interactable/Ammo/BP_AmmoPickupBase.PickupAmmo` _asbp_ammo_pickup_base))))
        (:`then_1`
          (bind _asbp_weapon_pickup_base (cast `/Game/FPSGame/Interactable/Weapons/BP_WeaponPickupBase` _hitactor))
          (`/Game/FPSGame/Interactable/Weapons/BP_WeaponPickupBase.InteractedWithWeapon` _asbp_weapon_pickup_base))))))

(event `InputAction|Fire`
  (params (Key :type "Key Structure"))
  ;[0.5 0 0] To shoot using right click
  (:`Pressed`
    (switch `/Game/FPSGame/Data/E_Loadout` (`self.Loadout`)
      (:`NewEnumerator1`
        (if (not (`self.isWeaponFireLoading?`))
          (if (`self.isSprinting?`)
            (`self.MovementStopped`))
          (`self.Fire`)))))
  (:`Released`
    (switch `/Game/FPSGame/Data/E_Loadout` (`self.Loadout`)
      (:`NewEnumerator1`
        (`/Game/FPSGame/Weapons/BP_WeaponBase.StopShooting` (`self.CurrentWeapon`))))))

(event `InputAction|Reload`
  (params (Key :type "Key Structure"))
  (:`Pressed`
    (switch `/Game/FPSGame/Data/E_Loadout` (`self.Loadout`)
      (:`NewEnumerator1`
        (bind _returnvalue (`/Game/FPSGame/Weapons/BP_WeaponBase.isMagFull orEmpty?` (`self.CurrentWeapon`)))
        (if _returnvalue
          (if (`self.isSprinting?`)
            (`self.MovementStopped`))
          ;[0.5 0 0] Stops gun from shooting while reload
          (if (`/Game/FPSGame/Weapons/BP_WeaponBase.isFiring?` (`self.CurrentWeapon`))
            (`/Game/FPSGame/Weapons/BP_WeaponBase.StopShooting` (`self.CurrentWeapon`)))
          (`self.Reload`))))))

(event `InputAction|Aim`
  (params (Key :type "Key Structure"))
  (bind _loadout (`self.Loadout`))
  (bind _charactermovement (`self.CharacterMovement`))
  (:`Pressed`
    (if (not (`self.isReloading?`))
      (set `self.IsAiming?` true)
      (`self.AimEnter`)
      (`self.MovementStopped`)
      ;[0.5 0 0] Slows player down when aiming
      (switch `/Game/FPSGame/Data/E_Loadout` _loadout
        (:`NewEnumerator1`
          (set `CharacterMovementComponent.MaxWalkSpeed` (`self.AimingWalkSpeed`) _charactermovement)))))
  (:`Released`
    (set `self.IsAiming?` false)
    (`self.AimExit`)
    (switch `/Game/FPSGame/Data/E_Loadout` _loadout
      (:`NewEnumerator1`
        (set `CharacterMovementComponent.MaxWalkSpeed` (`self.Max Walk Speed`) _charactermovement)))))

(fn `AimFieldOfView`
  (if (`self.IsAiming?`)
    ;[0.5 0 0] Changes FOV if aiming weapon
    (`CameraComponent.SetFieldOfView` (`self.Camera`) (`KismetMathLibrary.FInterpTo` (`CameraComponent.FieldOfView` (`self.Camera`)) (`/Game/FPSGame/Weapons/BP_WeaponBase.AimFieldOfView` (`self.CurrentWeapon`)) (`GameplayStatics.GetWorldDeltaSeconds`) 10.0))
    (else
      (`CameraComponent.SetFieldOfView` (`self.Camera`) (`KismetMathLibrary.FInterpTo` (`CameraComponent.FieldOfView` (`self.Camera`)) 90.0 (`GameplayStatics.GetWorldDeltaSeconds`) 10.0)))))

(fn `HideAndShowWeaponMesh`
  (params (Weapon :type "/Game/FPSGame/Weapons/BP_WeaponBase Object Reference"))
  (locals (LocalCurrentWeapon :type "/Game/FPSGame/Weapons/BP_WeaponBase Object Reference"))
  (bind _weaponslot05 (`self.WeaponSlot05`))
  (bind _weaponslot01 (`self.WeaponSlot01`))
  (bind _weaponslot06 (`self.WeaponSlot06`))
  (bind _weaponslot02 (`self.WeaponSlot02`))
  (bind _weaponslot03 (`self.WeaponSlot03`))
  (bind _weaponslot04 (`self.WeaponSlot04`))
  (set `local.LocalCurrentWeapon` Weapon)
  ;[0.5 0 0] Hide Currently equipped weapon
  (`/Engine/EditorBlueprintResources/StandardMacros.IsValid` _weaponslot01
    (:`Is Valid`
      (`self.SetActorHiddenInGame` _weaponslot01 true))
    (:`Is Not Valid`
      _))
  (`/Engine/EditorBlueprintResources/StandardMacros.IsValid` _weaponslot02
    (:`Is Valid`
      (`self.SetActorHiddenInGame` _weaponslot02 true))
    (:`Is Not Valid`
      _))
  (`/Engine/EditorBlueprintResources/StandardMacros.IsValid` _weaponslot03
    (:`Is Valid`
      (`self.SetActorHiddenInGame` _weaponslot03 true))
    (:`Is Not Valid`
      _))
  (`/Engine/EditorBlueprintResources/StandardMacros.IsValid` _weaponslot04
    (:`Is Valid`
      (`self.SetActorHiddenInGame` _weaponslot04 true))
    (:`Is Not Valid`
      _))
  (`/Engine/EditorBlueprintResources/StandardMacros.IsValid` _weaponslot05
    (:`Is Valid`
      (`self.SetActorHiddenInGame` _weaponslot05 true))
    (:`Is Not Valid`
      _))
  (`/Engine/EditorBlueprintResources/StandardMacros.IsValid` _weaponslot06
    (:`Is Valid`
      (`self.SetActorHiddenInGame` _weaponslot06 true))
    (:`Is Not Valid`
      _))
  ;[0.5 0 0] Show the mesh of the currently equipped weapon
  (if (== (`local.LocalCurrentWeapon`) (`self.WeaponSlot01`))
    (`self.SetActorHiddenInGame` (`self.WeaponSlot01`) false)
    (elif (== (`local.LocalCurrentWeapon`) (`self.WeaponSlot02`))
      (`self.SetActorHiddenInGame` (`self.WeaponSlot02`) false)
      (elif (== (`local.LocalCurrentWeapon`) (`self.WeaponSlot03`))
        (`self.SetActorHiddenInGame` (`self.WeaponSlot03`) false)
        (elif (== (`local.LocalCurrentWeapon`) (`self.WeaponSlot04`))
          (`self.SetActorHiddenInGame` (`self.WeaponSlot04`) false)
          (elif (== (`local.LocalCurrentWeapon`) (`self.WeaponSlot05`))
            (`self.SetActorHiddenInGame` (`self.WeaponSlot05`) false)
            (elif (== (`local.LocalCurrentWeapon`) (`self.WeaponSlot06`))
              (`self.SetActorHiddenInGame` (`self.WeaponSlot06`) false))))))))

(fn `SpawnWeapon`
  (params (Weapon :type "/Game/FPSGame/Weapons/BP_WeaponBase Class Reference"))
  (returns (ReturnWeapon :type "/Game/FPSGame/Weapons/BP_WeaponBase Object Reference"))
  (locals (LocalWeapon :type "/Game/FPSGame/Weapons/BP_WeaponBase Class Reference"))
  ;[0.5 0 0] Spawns Weapon actor in playrs hand and assigns slot
  (set `local.LocalWeapon` Weapon)
  (if (not (`self.Is1stSlotFilled?`))
    (bind _returnvalue (`|SpawnActorFromClass` (`local.LocalWeapon`) (`self.GetTransform`) "Undefined" "OverrideRootScale" null null))
    (bind _output_get (set `self.WeaponSlot01` _returnvalue))
    (set `self.Is1stSlotFilled?` true)
    (`self.K2_AttachToComponent` _output_get (`self.PlayerArms`) (`/Game/FPSGame/Weapons/BP_WeaponBase.SocketName` _returnvalue) "SnapToTarget" "SnapToTarget" "SnapToTarget" false)
    (bind _output_get_2 (set `self.CurrentWeapon` _output_get))
    (return _output_get_2)
    (elif (not (`self.Is2ndSlotFilled?`))
      (bind _returnvalue_2 (`|SpawnActorFromClass` (`local.LocalWeapon`) (`self.GetTransform`) "Undefined" "OverrideRootScale" null null))
      (bind _output_get_3 (set `self.WeaponSlot02` _returnvalue_2))
      (set `self.Is2ndSlotFilled?` true)
      (`self.K2_AttachToComponent` _output_get_3 (`self.PlayerArms`) (`/Game/FPSGame/Weapons/BP_WeaponBase.SocketName` _returnvalue_2) "SnapToTarget" "SnapToTarget" "SnapToTarget" false)
      (bind _output_get_4 (set `self.CurrentWeapon` _output_get_3))
      (return _output_get_4)
      (elif (not (`self.Is3rdSlotFilled?`))
        (bind _returnvalue_3 (`|SpawnActorFromClass` (`local.LocalWeapon`) (`self.GetTransform`) "Undefined" "OverrideRootScale" null null))
        (bind _output_get_5 (set `self.WeaponSlot03` _returnvalue_3))
        (set `self.Is3rdSlotFilled?` true)
        (`self.K2_AttachToComponent` _output_get_5 (`self.PlayerArms`) (`/Game/FPSGame/Weapons/BP_WeaponBase.SocketName` _returnvalue_3) "SnapToTarget" "SnapToTarget" "SnapToTarget" false)
        (bind _output_get_6 (set `self.CurrentWeapon` _output_get_5))
        (return _output_get_6)
        (elif (not (`self.Is4thSlotFilled?`))
          (bind _returnvalue_4 (`|SpawnActorFromClass` (`local.LocalWeapon`) (`self.GetTransform`) "Undefined" "OverrideRootScale" null null))
          (bind _output_get_7 (set `self.WeaponSlot04` _returnvalue_4))
          (set `self.Is4thSlotFilled?` true)
          (`self.K2_AttachToComponent` _output_get_7 (`self.PlayerArms`) (`/Game/FPSGame/Weapons/BP_WeaponBase.SocketName` _returnvalue_4) "SnapToTarget" "SnapToTarget" "SnapToTarget" false)
          (bind _output_get_8 (set `self.CurrentWeapon` _output_get_7))
          (return _output_get_8)
          (elif (not (`self.Is5thSlotFilled?`))
            (bind _returnvalue_5 (`|SpawnActorFromClass` (`local.LocalWeapon`) (`self.GetTransform`) "Undefined" "OverrideRootScale" null null))
            (bind _output_get_9 (set `self.WeaponSlot05` _returnvalue_5))
            (set `self.Is5thSlotFilled?` true)
            (`self.K2_AttachToComponent` _output_get_9 (`self.PlayerArms`) (`/Game/FPSGame/Weapons/BP_WeaponBase.SocketName` _returnvalue_5) "SnapToTarget" "SnapToTarget" "SnapToTarget" false)
            (bind _output_get_10 (set `self.CurrentWeapon` _output_get_9))
            (return _output_get_10)
            (elif (not (`self.Is6thSlotFilled?`))
              (bind _returnvalue_6 (`|SpawnActorFromClass` (`local.LocalWeapon`) (`self.GetTransform`) "Undefined" "OverrideRootScale" null null))
              (bind _output_get_11 (set `self.WeaponSlot06` _returnvalue_6))
              (set `self.Is6thSlotFilled?` true)
              (`self.K2_AttachToComponent` _output_get_11 (`self.PlayerArms`) (`/Game/FPSGame/Weapons/BP_WeaponBase.SocketName` _returnvalue_6) "SnapToTarget" "SnapToTarget" "SnapToTarget" false)
              (bind _output_get_12 (set `self.CurrentWeapon` _output_get_11))
              (return _output_get_12))))))))

(fn `StartSprint`
  (if (not (`NavMovementComponent.IsFalling` (`self.CharacterMovement`)))
    (set `CharacterMovementComponent.MaxWalkSpeed` (`self.SprintSpeed`) (`self.CharacterMovement`))
    (set `self.isSprinting?` true)))

(fn `StopSprint`
  (set `CharacterMovementComponent.MaxWalkSpeed` (`self.Max Walk Speed`) (`self.CharacterMovement`))
  (set `self.isSprinting?` false))

(fn `UserConstructionScript`)